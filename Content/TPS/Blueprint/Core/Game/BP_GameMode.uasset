(event `self.ReceiveBeginPlay`
  (`KismetSystemLibrary.K2_SetTimer` null "TryRespawnEnemy" 1.0 true))

(event `self.HandleStartingNewPlayer`
  (params (NewPlayer :type "PlayerController Object Reference"))
  (`parent.HandleStartingNewPlayer` NewPlayer)
  (`KismetArrayLibrary.Array_Add` (`self.Controllers`) NewPlayer)
  (bind _asbp_game_instance (cast `/Game/TPS/Blueprint/Core/Game/BP_GameInstance` (`GameplayStatics.GetGameInstance`)))
  (bind _asbp_player_controller (cast `/Game/TPS/Blueprint/Core/Game/BP_PlayerController` NewPlayer))
  (set `/Game/TPS/Blueprint/Core/Game/BP_PlayerController.PlayerColor` (`BlueprintMapLibrary.Map_Find` (`/Game/TPS/Blueprint/Core/Game/BP_GameInstance.ColorForPlayers` _asbp_game_instance) (`PlayerState.GetPlayerName` (`Controller.PlayerState` NewPlayer))) _asbp_player_controller))

(event `self.K2_OnLogout`
  (params (ExitingController :type "Controller Object Reference"))
  (`KismetArrayLibrary.Array_RemoveItem` (`self.Controllers`) ExitingController))

(event `RestartLevel`
  (for _array_element (`self.Controllers`)
    (bind _asbp_player_controller (cast `/Game/TPS/Blueprint/Core/Game/BP_PlayerController` _array_element))
    (`/Game/TPS/Blueprint/Core/Game/BP_PlayerController.UnbindWidgetEvents` _asbp_player_controller null))
  (bind _returnvalue (`GameplayStatics.GetCurrentLevelName` true))
  (`KismetSystemLibrary.ExecuteConsoleCommand` (`KismetStringLibrary.Concat_StrStr` "ServerTravel" " " _returnvalue) null))

(fn `BossDead`
  (`self.End Game_GameMode` true))

(fn `ChoosePlayerStart`
  (params (Player :type "Controller Object Reference"))
  (returns (ReturnValue :type "Actor Object Reference"))
  (return (`self.K2_FindPlayerStart` Player "Phase1")))

(fn `End Game_GameMode`
  (params (bIsWin :type Boolean))
  (for _array_element (`self.Controllers`)
    (bind _asbp_player_controller (cast `/Game/TPS/Blueprint/Core/Game/BP_PlayerController` _array_element))
    (`/Game/TPS/Blueprint/Core/Game/BP_PlayerController.EndGame_PlayerController` _asbp_player_controller bIsWin))
  (`KismetSystemLibrary.K2_SetTimer` null "PauseGame" 4.0))

(fn `EnemyDead`
  (params (Score :type Integer))
  (if (> Score 0)
    (bind _asbp_game_state (cast `/Game/TPS/Blueprint/Core/Game/BP_GameState` (`GameplayStatics.GetGameState`)))
    (bind _biswin (`/Game/TPS/Blueprint/Core/Game/BP_GameState.Increment Score` _asbp_game_state Score))
    (`/Game/TPS/Blueprint/Core/Game/BP_GameState.IncrementEnemy` _asbp_game_state -1)
    (if _biswin
      (`self.End Game_GameMode` true))))

(fn `NextPhaseStart`
  (params (CurrentPhase :type Integer))
  (bind _outactors (`GameplayStatics.GetAllActorsOfClass` "/Game/TPS/Blueprint/EnemyCharacter/BP_CharacterEnemy_Base.BP_CharacterEnemy_Base_C"))
  (for _array_element _outactors
    (bind _returnvalue (`TPSHealthComponent.GetIsAlive` (`/Game/TPS/Blueprint/EnemyCharacter/BP_CharacterEnemy_Base.TPSHealth` _array_element)))
    (if _returnvalue
      (`/Game/TPS/Blueprint/BP_KillScoreComponent.Destroy` (`/Game/TPS/Blueprint/EnemyCharacter/BP_CharacterEnemy_Base.BP_KillScoreComponent` _array_element)))))

(fn `PauseGame`
  (`GameplayStatics.SetGamePaused` true))

(fn `TryRespawnEnemy`
  (locals (CurrentPoint :type "/Game/TPS/Blueprint/EnemySpawner/EnemySpawn Object Reference"))
  (bind _asbp_game_state (cast `/Game/TPS/Blueprint/Core/Game/BP_GameState` (`GameplayStatics.GetGameState`)))
  (bind _valid (`/Game/TPS/Blueprint/Core/Game/BP_GameState.CheckEnemyForPhase` _asbp_game_state))
  (if _valid
    (bind _returnvalue (select `int` (`/Game/TPS/Blueprint/Core/Game/BP_GameState.CurrentPhase` _asbp_game_state) :`0` (`self.SpawnPointPhase1`) :`1` (`self.SpawnPointPhase2`) :`2` (`self.SpawnPointPhase3`) :`3` (`self.SpawnPointPhase4`) :`4` (`self.SpawnPointPhase5`)))
    (bind _output_get (set `local.CurrentPoint` (`|GetArrayItem` _returnvalue (`KismetMathLibrary.RandomIntegerInRange` 0 (- (`KismetArrayLibrary.Array_Length` _returnvalue) 1)))))
    (if (`/Game/TPS/Blueprint/EnemySpawner/EnemySpawn.bIsPoint` _output_get)
      (bind _returnvalue_2 (`self.K2_GetActorLocation` _output_get))
      (`|SpawnActorFromClass` "/Game/TPS/Blueprint/EnemyCharacter/BP_CharacterEnemy_Base.BP_CharacterEnemy_Base_C" (`KismetMathLibrary.Conv_VectorToTransform` _returnvalue_2) "AdjustIfPossibleButDontSpawnIfColliding" "OverrideRootScale" null null)
      (else
        (`|SpawnActorFromClass` "/Game/TPS/Blueprint/EnemyCharacter/BP_CharacterEnemy_Base.BP_CharacterEnemy_Base_C" (`KismetMathLibrary.Conv_VectorToTransform` (`KismetMathLibrary.RandomPointInBoundingBox` _returnvalue_2 (`BoxComponent.BoxExtent` (`/Game/TPS/Blueprint/EnemySpawner/EnemySpawn.Box` _output_get)))) "AdjustIfPossibleButDontSpawnIfColliding" "OverrideRootScale" null null)))
    (`/Game/TPS/Blueprint/Core/Game/BP_GameState.IncrementEnemy` _asbp_game_state 1)))

(fn `TrySpawnBoss`
  (params (ClassBoss :type "Pawn Class Reference"))
  (bind _returnvalue (`|SpawnActorFromClass` ClassBoss (`KismetMathLibrary.Conv_VectorToTransform` (`self.K2_GetActorLocation` (`self.SpawnPointBoss`))) "AdjustIfPossibleButAlwaysSpawn" "OverrideRootScale" null null))
  (bind _asbp_character_enemy_boss (cast `/Game/TPS/Blueprint/EnemyCharacter/Boss/BP_CharacterEnemy_Boss` _returnvalue))
  (add `TPSHealthComponent.OnDead` (`/Game/TPS/Blueprint/EnemyCharacter/BP_CharacterEnemy_Base.TPSHealth` _asbp_character_enemy_boss) (`|CreateDelegate` :!event `BossDead`)))

(fn `TryToRespawnPlayer`
  (params (DeadController :type "/Game/TPS/Blueprint/Core/Game/BP_PlayerController Object Reference"))
  (returns (Success :type Boolean))
  (bind _asbp_game_state (cast `/Game/TPS/Blueprint/Core/Game/BP_GameState` (`GameplayStatics.GetGameState`)))
  (bind (_success _currentphase) (`/Game/TPS/Blueprint/Core/Game/BP_GameState.CanPlayerRespawn` _asbp_game_state))
  (if _success
    (`self.RestartPlayerAtPlayerStart` DeadController (`self.K2_FindPlayerStart` DeadController (select `int` _currentphase :`0` "Phase0" :`1` "Phase1" :`2` "Phase2" :`3` "Phase3" :`4` "Phase4")))
    (return true)
    (else
      (return _success))))

(fn `TryToRespawnPlkayerAtSpectrator`
  (params (PlayerControllerDied :type "/Game/TPS/Blueprint/Core/Game/BP_PlayerController Object Reference"))
  (locals (TargetForSpectator :type "/Game/TPS/Blueprint/Character/BP_Character Object Reference"))
  (bind _targetforspectator (`local.TargetForSpectator`))
  (for _array_element (`self.Controllers`)
    (bind _asbp_character (cast `/Game/TPS/Blueprint/Character/BP_Character` (`Controller.K2_GetPawn` _array_element)))
    (if (`TPSCharacter.GetIsAlive` _asbp_character)
      (set `local.TargetForSpectator` _asbp_character)
      (break)))
  (`/Engine/EditorBlueprintResources/StandardMacros.IsValid` _targetforspectator
    (:`Is Valid`
      (bind _returnvalue (`|SpawnActorFromClass` "/Game/TPS/Blueprint/Core/Game/BP_PlayerSpectator.BP_PlayerSpectator_C" (`KismetMathLibrary.Conv_VectorToTransform` (`self.K2_GetActorLocation` _targetforspectator)) "AlwaysSpawn" "OverrideRootScale" null _targetforspectator null))
      (`Controller.Possess` PlayerControllerDied _returnvalue))
    (:`Is Not Valid`
      (`self.End Game_GameMode` false))))

(fn `UserConstructionScript`)
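; Player controller for a multiplayer third-person shooter that manages the in-game HUD, pawn setup and end-game screen.
; BeginPlay creates the HUD for local players and binds inventory and health widgets to BP_Character.
; Possess applies player color, restores inventory from BP_PlayerState and reinitializes widgets; UnPossess unbinds them, and OnRep_PlayerColor reapplies color.
; Escape toggles the end-game widget, and Left Ctrl toggles slow motion through global time dilation.
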(event `self.ReceiveBeginPlay`
  (`/Engine/EditorBlueprintResources/ActorMacros.Switch Has Authority`
    (:`Authority`
      (if (`self.IsLocalPlayerController`)
        (`GameplayStatics.PushSoundMixModifier` "/Game/TPS/Blueprint/Sounds/MIX_Main.MIX_Main" :!label _label)
        (bind _returnvalue (`|CreateWidget` "/Game/TPS/Blueprint/Widget/BPW_IngameWidget.BPW_IngameWidget_C" self))
        (bind _output_get (set `self.IngameWidget` _returnvalue))
        (`UserWidget.AddToViewport` _returnvalue 0)
        (bind _asbp_character (cast `/Game/TPS/Blueprint/Character/BP_Character` (`self.K2_GetPawn`)))
        (bind _inventorystatswidget (`/Game/TPS/Blueprint/Widget/BPW_IngameWidget.InventoryStatsWidget` _output_get))
        (`/Game/TPS/Blueprint/Widget/Inventory/BPW_InventoryStatsWidget.BindInventoryEvents` _inventorystatswidget _asbp_character)
        (bind _inventorycomponent (`TPSCharacter.InventoryComponent` _asbp_character))
        (`/Game/TPS/Blueprint/Widget/Inventory/BPW_InventoryStatsWidget.InitInventorySlots` _inventorystatswidget (`TPSInventoryComponent.WeaponSlots` _inventorycomponent) (`TPSInventoryComponent.AmmoSlots` _inventorycomponent))
        (`/Game/TPS/Blueprint/Widget/Health/BPW_StatsCharacterBar.Init Widget` (`/Game/TPS/Blueprint/Widget/BPW_IngameWidget.HealthBar` _output_get) _asbp_character)))
    (:`Remote`
      (goto _label))))

(event `self.ReceiveTick`
  (params (DeltaSeconds :type "Float (single-precision)")))

(event `Key|LeftControl`
  (params (Key :type "Key Structure"))
  (:`Pressed`
    (`/Engine/EditorBlueprintResources/StandardMacros.FlipFlop`
      (:`A`
        (`GameplayStatics.SetGlobalTimeDilation` 0.1))
      (:`B`
        (`GameplayStatics.SetGlobalTimeDilation` 1.0)))))

(event `Key|Escape`
  (params (Key :type "Key Structure"))
  (bind _ingamewidget (`self.IngameWidget`))
  (bind _bpw_endgame (`/Game/TPS/Blueprint/Widget/BPW_IngameWidget.BPW_EndGame` _ingamewidget))
  (bind _returnvalue (`Widget.IsVisible` _bpw_endgame))
  (:`Pressed`
    (`/Engine/EditorBlueprintResources/StandardMacros.IsValid` _ingamewidget
      (:`Is Valid`
        (`Widget.SetVisibility` _bpw_endgame (select `bool` _returnvalue :`false` "Visible" :`true` "Collapsed" :!type "ESlateVisibility Enum"))
        (set `self.bShowMouseCursor` _returnvalue)))))

(event `self.ReceiveUnPossess`
  (params (UnpossessedPawn :type "Pawn Object Reference"))
  (`self.UnbindWidgetEvents` UnpossessedPawn))

(event `EndGame_PlayerController`
  (params (bIsWin :type Boolean))
  (bind _bpw_endgame (`/Game/TPS/Blueprint/Widget/BPW_IngameWidget.BPW_EndGame` (`self.IngameWidget`)))
  (set `self.bShowMouseCursor` true)
  (`Widget.SetVisibility` _bpw_endgame "Visible")
  (`/Game/TPS/Blueprint/Widget/BPW_EndGame.InitWidgetEndGame` _bpw_endgame bIsWin (`KismetSystemLibrary.IsServer`)))

(event `UnbindWidgetEvents`
  (params (Object :type "Object Object Reference"))
  (`self.UnbindWidgets` Object))

(event `UpdatePlayerColorPawn`
  (bind _asbp_character (cast `/Game/TPS/Blueprint/Character/BP_Character` (`self.K2_GetPawn`)))
  (`/Game/TPS/Blueprint/Character/BP_Character.SetColorCharacter_OnServer` _asbp_character (`self.PlayerColor`)))

(event `self.ReceivePossess`
  (params (PossessedPawn :type "Pawn Object Reference"))
  (bind _asbp_character (cast `/Game/TPS/Blueprint/Character/BP_Character` PossessedPawn))
  (`/Game/TPS/Blueprint/Character/BP_Character.SetColorCharacter_OnServer` _asbp_character (`self.PlayerColor`))
  (bind _asbp_player_state (cast `/Game/TPS/Blueprint/Core/Game/BP_PlayerState` (`self.PlayerState`)))
  (bind _weaponslots (`/Game/TPS/Blueprint/Core/Game/BP_PlayerState.WeaponSlots` _asbp_player_state))
  (bind _ammoslots (`/Game/TPS/Blueprint/Core/Game/BP_PlayerState.AmmoSlots` _asbp_player_state))
  (`TPSInventoryComponent.InitInventory_OnServer` (`TPSCharacter.InventoryComponent` _asbp_character) _weaponslots _ammoslots)
  (`self.InitWidget` _weaponslots _ammoslots))

(event `InitWidget`
  (params (Weapons :type "Array of WeaponSlot Structure (by ref)") (Ammo :type "Array of AmmoSlot Structure (by ref)"))
  (bind _ingamewidget (`self.IngameWidget`))
  (bind _inventorystatswidget (`/Game/TPS/Blueprint/Widget/BPW_IngameWidget.InventoryStatsWidget` _ingamewidget))
  (`/Engine/EditorBlueprintResources/StandardMacros.IsValid` _ingamewidget
    (:`Is Valid`
      (bind _asbp_character (cast `/Game/TPS/Blueprint/Character/BP_Character` (`self.K2_GetPawn`)))
      (`/Game/TPS/Blueprint/Widget/Inventory/BPW_InventoryStatsWidget.BindInventoryEvents` _inventorystatswidget _asbp_character)
      (`/Game/TPS/Blueprint/Widget/Inventory/BPW_InventoryStatsWidget.InitInventorySlots` _inventorystatswidget Weapons Ammo)
      (`/Game/TPS/Blueprint/Widget/Health/BPW_StatsCharacterBar.Init Widget` (`/Game/TPS/Blueprint/Widget/BPW_IngameWidget.HealthBar` _ingamewidget) _asbp_character))))

(fn `OnRep_PlayerColor`
  (`self.UpdatePlayerColorPawn`))

(fn `UnbindWidgets`
  (params (Target :type "Object Object Reference"))
  (locals (myTarget :type "Object Object Reference"))
  (bind _ingamewidget (`self.IngameWidget`))
  (`/Engine/EditorBlueprintResources/StandardMacros.IsValid` Target
    (:`Is Valid`
      (set `local.myTarget` Target))
    (:`Is Not Valid`
      (set `local.myTarget` (`self.K2_GetPawn`))))
  (`/Engine/EditorBlueprintResources/StandardMacros.IsValid` _ingamewidget
    (:`Is Valid`
      (`Widget.SetVisibility` (`/Game/TPS/Blueprint/Widget/BPW_IngameWidget.BPW_EndGame` _ingamewidget) "Collapsed")
      (`Widget.SetVisibility` (`/Game/TPS/Blueprint/Widget/BPW_IngameWidget.BPW_PickUpWidget` _ingamewidget) "Collapsed")
      (bind _asbp_character (cast `/Game/TPS/Blueprint/Character/BP_Character` (`local.myTarget`)))
      (`/Game/TPS/Blueprint/Widget/Inventory/BPW_InventoryStatsWidget.UnbindAllEvents` (`/Game/TPS/Blueprint/Widget/BPW_IngameWidget.InventoryStatsWidget` _ingamewidget) _asbp_character)
      (`/Game/TPS/Blueprint/Widget/Health/BPW_StatsCharacterBar.UnBindWidget` (`/Game/TPS/Blueprint/Widget/BPW_IngameWidget.HealthBar` _ingamewidget)))))

(fn `UserConstructionScript`)
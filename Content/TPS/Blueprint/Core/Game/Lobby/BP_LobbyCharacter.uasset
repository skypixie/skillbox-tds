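; Lobby character whose skeletal mesh shows a selectable color material and plays a stretch montage as a ready signal.
; A server color-change event forwards the material to a multicast, which sets it on the first mesh slot and stores it as CurrentColor.
; Non-authority instances reapply CurrentColor on BeginPlay, and the ready multicast event plays the montage.
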(event `ChangeColor_OnServer`
  (params (Material :type "MaterialInterface Object Reference"))
  (`self.ChangeColor_Multicast` Material))

(event `ChangeColor_Multicast`
  (params (Material :type "MaterialInterface Object Reference"))
  (`PrimitiveComponent.SetMaterial` (`self.SkeletalMesh`) 0 Material)
  (set `self.CurrentColor` Material))

(event `self.ReceiveBeginPlay`
  (`/Engine/EditorBlueprintResources/ActorMacros.Switch Has Authority`
    (:`Remote`
      (`PrimitiveComponent.SetMaterial` (`self.SkeletalMesh`) 0 (`self.CurrentColor`)))))

(event `self.ReceiveTick`
  (params (DeltaSeconds :type "Float (single-precision)")))

(event `MeReady_Multicast`
  (`|PlayMontage` (`self.SkeletalMesh`) "/Game/TPS/Characters/PlayerCharacter/Animations/Emotion/Anim_Body_Stretch_2_Montage.Anim_Body_Stretch_2_Montage"))

(fn `UserConstructionScript`)
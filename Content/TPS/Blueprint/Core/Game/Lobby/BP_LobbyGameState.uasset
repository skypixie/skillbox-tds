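; Lobby GameState that tracks which colors are blocked and which remain available for players.
; Server events swap, add or remove entries in BlockColors, then loop through BP_LobbyMode's player controllers to push the list to each client's lobby widget.
; Getters return the blocked colors or filter AllColors down to the available ones.
; The BlockColors RepNotify is empty, so UI updates rely on those explicit controller calls.
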(event `SelectedNewColor_OnServer`
  (params (Remove :type "MaterialInterface Object Reference") (Add :type "MaterialInterface Object Reference"))
  (bind _blockcolors (`self.BlockColors`))
  (`KismetArrayLibrary.Array_RemoveItem` _blockcolors Remove)
  (`KismetArrayLibrary.Array_Add` _blockcolors Add)
  (bind _asbp_lobby_mode (cast `/Game/TPS/Blueprint/Core/Game/Lobby/BP_LobbyMode` (`GameplayStatics.GetGameMode`)))
  (for _array_element (`/Game/TPS/Blueprint/Core/Game/Lobby/BP_LobbyMode.PlayerControllers` _asbp_lobby_mode)
    (bind _asbp_lobby_player_controller (cast `/Game/TPS/Blueprint/Core/Game/Lobby/BP_LobbyPlayerController` _array_element))
    (`/Game/TPS/Blueprint/Core/Game/Lobby/BP_LobbyPlayerController.UpdateColorsLobbyWidget_OnClient` _asbp_lobby_player_controller (`self.BlockColors`))))

(event `AddOrRemoveColorToBlock_OnServer`
  (params (Color :type "MaterialInterface Object Reference") (bIsRemove :type Boolean))
  (bind _blockcolors (`self.BlockColors`))
  (if bIsRemove
    (`KismetArrayLibrary.Array_RemoveItem` _blockcolors Color)
    (else
      (`KismetArrayLibrary.Array_Add` _blockcolors Color)))
  (bind _asbp_lobby_mode (cast `/Game/TPS/Blueprint/Core/Game/Lobby/BP_LobbyMode` (`GameplayStatics.GetGameMode`)))
  (for _array_element (`/Game/TPS/Blueprint/Core/Game/Lobby/BP_LobbyMode.PlayerControllers` _asbp_lobby_mode)
    (bind _asbp_lobby_player_controller (cast `/Game/TPS/Blueprint/Core/Game/Lobby/BP_LobbyPlayerController` _array_element))
    (`/Game/TPS/Blueprint/Core/Game/Lobby/BP_LobbyPlayerController.UpdateColorsLobbyWidget_OnClient` _asbp_lobby_player_controller (`self.BlockColors`))))

(fn `GetAviableColors`
  (returns (AviableColorOut :type "Array of MaterialInterface Object Reference"))
  (locals (AviableColor :type "Array of MaterialInterface Object Reference") (TakeIt :type Boolean :default true))
  (for _array_element (`self.AllColors`)
    (set `local.TakeIt` true)
    (for _array_element_2 (`self.BlockColors`)
      (if (== _array_element_2 _array_element)
        (set `local.TakeIt` false)
        (break)))
    (if (`local.TakeIt`)
      (`KismetArrayLibrary.Array_Add` (`local.AviableColor`) _array_element)))
  (return (`local.AviableColor`)))

(fn `GetBlocksColors`
  (returns (AviableColors :type "Array of MaterialInterface Object Reference"))
  (locals (Colors :type "Array of MaterialInterface Object Reference"))
  (return (`self.BlockColors`)))

(fn `OnRep_BlockColors`)

(fn `UserConstructionScript`)
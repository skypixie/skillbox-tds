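; Base melee enemy character for a networked TPS, with health, attacks, hit reactions and ammo drops.
; Damage feeds TPSHealth, spawning floating damage numbers and server-rolled confusion, flinch or slowdown effects.
; Light and heavy attacks multicast random montages, whose "Attack" notifies run server sphere traces damaging Player-tagged actors, while flags gate movement and attacking.
; Death plays a montage, unpossesses, drops any randomly assigned weapon-type item, then ragdolls on the server.
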(event `self.ReceiveTick`
  (params (DeltaSeconds :type "Float (single-precision)"))
  (set `self.DeltaTime` DeltaSeconds)
  (`|ExecutionSequence`
    (:`then_0`
      (`self.ChangeSpeedByHit`))))

(event `PlayAnim_Multicast`
  (params (AnimMontage :type "AnimMontage Object Reference") (InPlayRate :type "Float (double-precision)" :default 1.0) (StartSectionName :type Name))
  (`self.PlayAnimMontage` AnimMontage InPlayRate StartSectionName))

(event `self.TPSHealth.OnHealthChange`
  (params (Health :type "Float (single-precision)") (Damage :type "Float (single-precision)"))
  (bind _returnvalue (`|SpawnActorFromClass` "/Game/TPS/Blueprint/InteractionEnvironment/DisplayDamage/BP_DisplayDamage.BP_DisplayDamage_C" (`KismetMathLibrary.MakeTransform` (+ (+ (`KismetMathLibrary.MakeVector` (`KismetMathLibrary.RandomFloatInRange` -20.0 20.0) (`KismetMathLibrary.RandomFloatInRange` -20.0 20.0)) (`self.SpawnOffsetLocalDamage`)) (`self.K2_GetActorLocation`))) "AlwaysSpawn" "OverrideRootScale" null null))
  (`/Game/TPS/Blueprint/InteractionEnvironment/DisplayDamage/BP_DisplayDamage.InitActor` _returnvalue Damage Health)
  (`/Engine/EditorBlueprintResources/ActorMacros.Switch Has Authority`
    (:`Authority`
      (if (> (`KismetMathLibrary.RandomFloat`) (`self.ConfusionChance`))
        (`self.ConfusionEnabledTimer`)
        (else
          (`self.HitAnim`)))
      (if (> (`KismetMathLibrary.RandomFloat`) (`self.SlowDownSpeedChance`))
        (set `self.SlowDownSpeed` true)
        (`KismetSystemLibrary.K2_SetTimerDelegate` (delegate `SlowDownDisabled`) 2.0)))))

(event `SlowDownDisabled`
  (set `self.SlowDownSpeed` false))

(event `self.TPSHealth.OnDead`
  (bind _deadsanim (`self.DeadsAnim`))
  (`/Engine/EditorBlueprintResources/ActorMacros.Switch Has Authority`
    (:`Authority`
      (set `self.SelectedDead` (`|GetArrayItem` _deadsanim (- (`KismetArrayLibrary.Array_Length` _deadsanim) 1)))
      (`self.DadEvent_Mulicast` (`self.SelectedDead`)))))

(event `DadEvent_Mulicast`
  (params (SelectedDead :type "AnimMontage Object Reference"))
  (bind _dropcomponent (`self.DropComponent`))
  (`/Engine/EditorBlueprintResources/ActorMacros.Switch Has Authority`
    (:`Authority`
      (`|PlayMontage` (`self.Mesh`) SelectedDead
        (:`then`
          (`MovementComponent.StopMovementImmediately` (`self.CharacterMovement`))
          (`Controller.UnPossess` (`self.GetController`))
          (`self.SetLifeSpan` 20.0)
          (`self.SetStateAttack` false)
          (`self.SetStateMovement` false)
          (`/Engine/EditorBlueprintResources/StandardMacros.IsValid` _dropcomponent
            (:`Is Valid`
              (`/Game/TPS/Blueprint/BP_DropItemComponent.Drop` _dropcomponent))))
        (:`OnCompleted`
          (`self.EnableRagdoll`))))
    (:`Remote`
      (`self.PlayAnimMontage` SelectedDead))))

(event `EnableRagdoll`
  (bind _mesh (`self.Mesh`))
  (`PrimitiveComponent.SetCollisionProfileName` _mesh "PhysicsActor" true)
  (`PrimitiveComponent.SetCollisionEnabled` _mesh "PhysicsOnly")
  (`PrimitiveComponent.SetCollisionResponseToChannel` (`self.CapsuleComponent`) "ECC_Pawn" "ECR_Ignore")
  (`PrimitiveComponent.SetCollisionResponseToChannel` _mesh "ECC_Pawn" "ECR_Ignore")
  (`PrimitiveComponent.SetCollisionObjectType` _mesh "ECC_PhysicsBody")
  (`PrimitiveComponent.SetSimulatePhysics` _mesh true))

(event `self.ReceiveAnyDamage`
  (params (Damage :type "Float (single-precision)") (DamageType :type "DamageType Object Reference") (InstigatedBy :type "Controller Object Reference") (DamageCauser :type "Actor Object Reference"))
  (`TPSHealthComponent.ChangeHealthValue_OnServer` (`self.TPSHealth`) (* Damage -1.0))
  (set `self.LastInstigator` InstigatedBy))

(event `self.ReceiveBeginPlay`
  (`self.InitDropComponent`))

(event `MeleeAttackLight_Multicast`
  (params (SelectedLightAttack :type "AnimMontage Object Reference"))
  (bind _baselightdamage (`self.BaseLightDamage`))
  (`/Engine/EditorBlueprintResources/ActorMacros.Switch Has Authority`
    (:`Authority`
      (bind _notifyname (`|PlayMontage` (`self.Mesh`) SelectedLightAttack)
        (:`OnCompleted`
          (`self.SetStateAttack` true :!label _label))
        (:`OnInterrupted`
          (goto _label))
        (:`OnNotifyBegin`
          (if (== _notifyname "Attack")
            (`self.MeleeTrace` 50.0 150.0 (`KismetMathLibrary.RandomFloatInRange` (- _baselightdamage 10.0) (+ _baselightdamage 20.0)) (`self.LightRadius`))))))
    (:`Remote`
      (`self.PlayAnimMontage` SelectedLightAttack))))

(event `/Game/TPS/Blueprint/EnemyCharacter/Common/BPI_Combat.MeleeAttackLight`
  (bind _lightattackanim (`self.LightAttackAnim`))
  (`self.SetStateAttack` false)
  (set `self.SelectedLightAttack` (`|GetArrayItem` _lightattackanim (`KismetMathLibrary.RandomInteger` (`KismetArrayLibrary.Array_Length` _lightattackanim))))
  (`self.MeleeAttackLight_Multicast` (`self.SelectedLightAttack`)))

(event `MeleeAttackHeavy_Multicast`
  (params (SelectedHeavyAttack :type "AnimMontage Object Reference"))
  (bind _baseheavydamage (`self.BaseHeavyDamage`))
  (`/Engine/EditorBlueprintResources/ActorMacros.Switch Has Authority`
    (:`Authority`
      (bind _notifyname (`|PlayMontage` (`self.Mesh`) SelectedHeavyAttack)
        (:`OnCompleted`
          (`self.SetStateMovement` true :!label _label_2)
          (goto _label))
        (:`OnInterrupted`
          (goto _label_2))
        (:`OnNotifyBegin`
          (if (== _notifyname "Attack")
            (`self.MeleeTrace` 50.0 (`self.EndHeavyTraceDistance`) (`KismetMathLibrary.RandomFloatInRange` (- _baseheavydamage 10.0) (+ _baseheavydamage 50.0)) (`self.HeavyRadius`))))))
    (:`Remote`
      (`self.PlayAnimMontage` SelectedHeavyAttack))))

(event `/Game/TPS/Blueprint/EnemyCharacter/Common/BPI_Combat.MeleeAttackHeavy`
  (bind _heavyattackanim (`self.HeavyAttackAnim`))
  (`self.SetStateAttack` false)
  (`self.SetStateMovement` false)
  (set `self.SelectedHeavyAttack` (`|GetArrayItem` _heavyattackanim (`KismetMathLibrary.RandomInteger` (`KismetArrayLibrary.Array_Length` _heavyattackanim))))
  (`self.MeleeAttackHeavy_Multicast` (`self.SelectedHeavyAttack`)))

(fn `CanAttack`
  (returns (isCanAttack :type Boolean))
  (return (`self.CanAttackPawn`)))

(fn `CanMove`
  (returns (bIsCanMove :type Boolean))
  (return (`self.CanMovePawn`)))

(fn `ConfusionDisabledTimer`
  (`self.SetStateMovement` true)
  (set `CharacterMovementComponent.MaxWalkSpeed` 400.0 (`self.CharacterMovement`)))

(fn `ConfusionEnabledTimer`
  (locals (CurrentMontage :type "AnimMontage Object Reference"))
  (bind _confusionanim (`self.ConfusionAnim`))
  (`self.SetStateMovement` false)
  (bind _output_get (set `local.CurrentMontage` (`|GetArrayItem` _confusionanim (`KismetMathLibrary.RandomIntegerInRange` 0 (- (`KismetArrayLibrary.Array_Length` _confusionanim) 1)))))
  (bind _returnvalue (`AnimSequenceBase.GetPlayLength` _output_get))
  (`KismetSystemLibrary.K2_SetTimer` null "ConfusionDisabledTimer" _returnvalue)
  (`self.PlayAnim_Multicast` (`local.CurrentMontage`))
  (set `CharacterMovementComponent.MaxWalkSpeed` 0.0 (`self.CharacterMovement`))
  (set `self.bIsConfused` true))

(fn `HitAnim`
  (if (`self.bIsConfused`)
    _
    (elif (> (`KismetMathLibrary.RandomFloat`) (`self.HitAnimChance`))
      (`self.PlayAnim_Multicast` "/Game/TPS/Characters/EnemyZombie/Type2/Anim/zombie_reaction_hit__2__Montage.zombie_reaction_hit__2__Montage"))))

(fn `InitDropComponent`
  (locals (cout :type Integer))
  (`/Engine/EditorBlueprintResources/ActorMacros.Switch Has Authority`
    (:`Authority`
      (if (> (`KismetMathLibrary.RandomFloat`) (`self.DropChance`))
        (bind _returnvalue (`AddComponent|NODE_AddBP_DropItemComponent-0`))
        (set `self.DropComponent` _returnvalue)
        (bind _output_get (set `/Game/TPS/Blueprint/BP_DropItemComponent.Type` (select `int` (`KismetMathLibrary.RandomIntegerInRange` 0 3) :`0` "RifleType" :`1` "ShotGunType" :`2` "SniperRifle" :`3` "GrenadeLauncher" :!type "EWeaponType Enum") _returnvalue))
        (`|ExecutionSequence`
          (:`then_0`
            (switch `EWeaponType` _output_get
              (:`RifleType`
                (set `local.cout` 30))
              (:`ShotGunType`
                (set `local.cout` 12))
              (:`SniperRifle`
                (set `local.cout` 6))
              (:`GrenadeLauncher`
                (set `local.cout` 2))))
          (:`then_1`
            (set `/Game/TPS/Blueprint/BP_DropItemComponent.Cout` (`local.cout`) _returnvalue)))))))

(fn `SetStateAttack`
  (params (CanAttack :type Boolean))
  (set `self.CanAttackPawn` CanAttack))

(fn `SetStateMovement`
  (params (CanMove :type Boolean))
  (set `self.CanMovePawn` CanMove))

(fn `UserConstructionScript`)
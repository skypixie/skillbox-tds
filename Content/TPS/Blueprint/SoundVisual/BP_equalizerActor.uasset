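; Equalizer actor that visualizes a sound wave's frequency spectrum as a row of scaling props.
; BeginPlay starts the audio and spawns the props along world X, tinting their material instances on a green-to-white gradient.
; Each Tick samples the spectrum of Wave at game time rather than audio playback position, with one band per prop.
; Each band's multiplied magnitude drives its prop's Z scale and material "Inte" parameter.
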(event `self.ReceiveBeginPlay`
  (`AudioComponent.Play` (`self.Audio`) 0.0)
  (for _index (range 101)
    (bind _returnvalue (`|SpawnActorFromClass` "/Game/TPS/Blueprint/SoundVisual/Props.Props_C" (`KismetMathLibrary.MakeTransform` (`KismetMathLibrary.MakeVector` (+ (.x (`self.K2_GetActorLocation`)) (* _index 37.5)) (.y (`self.K2_GetActorLocation`)) (.z (`self.K2_GetActorLocation`)))) "AlwaysSpawn" "OverrideRootScale" null null))
    (`KismetArrayLibrary.Array_Add` (`self.EQ`) _returnvalue)
    (bind (_returnvalue_x _returnvalue_y _returnvalue_z) (`KismetMathLibrary.BreakVector` (`KismetMathLibrary.VLerp` (0.0 1.0 0.0) (1.0 1.0 1.0) (`KismetMathLibrary.MapRangeClamped` (`KismetMathLibrary.Conv_IntToDouble` _index) 0.0 100.0 0.0 1.0))))
    (`MaterialInstanceDynamic.SetVectorParameterValue` (`/Game/TPS/Blueprint/SoundVisual/Props.Inst_m` _returnvalue) "Color" (make `LinearColor` _returnvalue_x _returnvalue_y _returnvalue_z 1.0))))

(event `self.ReceiveTick`
  (params (DeltaSeconds :type "Float (single-precision)"))
  (bind _outspectrum (`SoundVisualizationStatics.CalculateFrequencySpectrum` (`self.wave`) 0 (`KismetSystemLibrary.GetGameTimeInSeconds`) 0.1 (`KismetArrayLibrary.Array_Length` (`self.EQ`))))
  (set `self.Spectr` _outspectrum)
  (for (_array_element _array_index) (`self.EQ`)
    (bind _returnvalue (* (`KismetMathLibrary.Abs` (`|GetArrayItem` (`self.Spectr`) _array_index)) (`self.CoefMultFR`)))
    (`self.SetActorScale3D` _array_element (`KismetMathLibrary.MakeVector` 1.0 1.0 _returnvalue))
    (`MaterialInstanceDynamic.SetScalarParameterValue` (`/Game/TPS/Blueprint/SoundVisual/Props.Inst_m` _array_element) "Inte" (`KismetMathLibrary.MapRangeClamped` _returnvalue 0.0 10.0 0.0 1.0))))

(fn `UserConstructionScript`)